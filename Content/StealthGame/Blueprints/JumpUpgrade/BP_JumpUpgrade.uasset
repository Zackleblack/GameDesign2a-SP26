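; BP_JumpUpgrade is a pickup that grants the player a boot upgrade in the stealth game.
; It destroys itself on BeginPlay if DoesPlayerHave is set.
; When BP_ThirdPersonCharacterCustom overlaps Pickup, it calls BootUpgrade and SaveGameState on the character, then destroys itself.
; Later sequence branches play a shutter sound and spawn sparks at the mesh, with delayed emitter cleanup queued after the actor's destruction.
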(event OnComponentBeginOverlap(Pickup)
  (params (OverlappedComponent :type Primitive%20Component%20Object%20Reference) (OtherActor :type Actor%20Object%20Reference) (OtherComp :type Primitive%20Component%20Object%20Reference) (OtherBodyIndex :type Integer) (bFromSweep :type Boolean) (SweepResult :type Hit%20Result%20Structure%20%28by%20ref%29))
  (bind _staticmesh (Variables|Default|GetStaticMesh))
  (bind _returnvalue (Transformation|GetWorldLocation _staticmesh))
  (bind _asbp_third_person_character_custom (Utilities|Casting|CastToBP_ThirdPersonCharacterCustom OtherActor))
  (Utilities|FlowControl|Sequence
    (:then_0
      (Default|BootUpgrade _asbp_third_person_character_custom)
      (Default|SaveGameState _asbp_third_person_character_custom)
      (Actor|DestroyActor))
    (:then_1
      (bind _returnvalue_2 (Effects|SpawnEmitteratLocation "/Game/StealthGame/Core/StarterContent/Particles/P_Sparks.P_Sparks" _returnvalue))
      (Utilities|FlowControl|Delay 1.0)
      (Components|DestroyComponent _returnvalue_2))
    (:then_2
      (Audio|PlaySoundatLocation "/Engine/VREditor/Sounds/UI/Camera_Shutter.Camera_Shutter" _returnvalue "0, 0, 0" 1.0 1.0 0.0 0 0 0 0))))

(event EventBeginPlay
  (if (Variables|Default|GetbDoesPlayerHave?)
    (Actor|DestroyActor)))

(fn ConstructionScript)