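; BP_ViewVent is an interactable vent that switches the player's view from the character to the vent.
; Box overlap with the custom third-person character tracks presence and shows or removes a W_PressE prompt.
; Interact fades the camera out, retargets the view to ViewPoint's owner, then fades in.
; Leaving the box after interacting returns the view to the character with the same fade, disabling character input meanwhile.
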(event OnComponentBeginOverlap(Box)
  (params (OverlappedComponent :type Primitive%20Component%20Object%20Reference) (OtherActor :type Actor%20Object%20Reference) (OtherComp :type Primitive%20Component%20Object%20Reference) (OtherBodyIndex :type Integer) (bFromSweep :type Boolean) (SweepResult :type Hit%20Result%20Structure%20%28by%20ref%29))
  (Utilities|Casting|CastToBP_ThirdPersonCharacterCustom OtherActor)
  (Variables|Default|SetbIsPlayerOn? true)
  (bind _returnvalue (UserInterface|CreateWidget "/Game/StealthGame/Core/Characters/PlayerCharacter/W_PressE.W_PressE_C"))
  (UserInterface|Viewport|AddtoViewport _returnvalue 0))

(event OnComponentEndOverlap(Box)
  (params (OverlappedComponent :type Primitive%20Component%20Object%20Reference) (OtherActor :type Actor%20Object%20Reference) (OtherComp :type Primitive%20Component%20Object%20Reference) (OtherBodyIndex :type Integer))
  (bind _returnvalue (Game|GetPlayerCameraManager 0))
  (bind _asbp_third_person_character_custom (Utilities|Casting|CastToBP_ThirdPersonCharacterCustom OtherActor))
  (Variables|Default|SetbIsPlayerOn? false)
  (Widget|RemovefromParent (stale OnComponentBeginOverlap(Box) _returnvalue))
  (if (Variables|Default|GetbDidPlayerInteract?)
    (Input|DisableInput _asbp_third_person_character_custom 0)
    (CameraFades|StartCameraFade :self _returnvalue :ToAlpha 1.0 :Duration 1.0 :bHoldWhenFinished true)
    (Utilities|FlowControl|Delay 2.0)
    (Game|Player|SetViewTargetwithBlend (Game|GetPlayerController 0) OtherActor 0.0 "VTBlend_Linear" 1.0 false)
    (CameraFades|StartCameraFade :self _returnvalue :FromAlpha 1.0 :Duration 1.0 :bHoldWhenFinished true)
    (Variables|Default|SetbDidPlayerInteract? false)
    (Input|EnableInput _asbp_third_person_character_custom (Game|GetPlayerController 0))))

(event EventInteract
  (bind _returnvalue (Game|GetPlayerCameraManager 0))
  (if (Variables|Default|GetbIsPlayerOn?)
    (Variables|Default|SetbDidPlayerInteract? true)
    (Widget|RemovefromParent (stale OnComponentBeginOverlap(Box) _returnvalue))
    (Input|DisableInput self (Game|GetPlayerController 0))
    (CameraFades|StartCameraFade :self _returnvalue :ToAlpha 1.0 :Duration 1.0 :bHoldWhenFinished true)
    (Utilities|FlowControl|Delay 2.0)
    (Game|Player|SetViewTargetwithBlend (Game|GetPlayerController 0) (Components|GetOwner (Variables|Default|GetView%20Point)) 0.0 "VTBlend_Linear" 1.0 false)
    (CameraFades|StartCameraFade :self _returnvalue :FromAlpha 1.0 :Duration 1.0 :bHoldWhenFinished true)
    (Input|EnableInput self (Game|GetPlayerController 0))))

(fn ConstructionScript)