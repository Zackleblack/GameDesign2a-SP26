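; BP_LibraryDoor is a key-locked door that swings open and closed on interaction.
; PickUpKey sets HasKey, which lets Interact use a FlipFlop to play or reverse a timeline that lerps the door's yaw.
; A Box overlap shows the player character either an open-door or need-key widget based on HasKey, then removes it on exit.
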(event OnComponentBeginOverlap(Box)
  (params (OverlappedComponent :type Primitive%20Component%20Object%20Reference) (OtherActor :type Actor%20Object%20Reference) (OtherComp :type Primitive%20Component%20Object%20Reference) (OtherBodyIndex :type Integer) (bFromSweep :type Boolean) (SweepResult :type Hit%20Result%20Structure%20%28by%20ref%29))
  (Utilities|Casting|CastToBP_ThirdPersonCharacterCustom OtherActor)
  (if (Variables|Default|GetbHasKey?)
    (bind _returnvalue (UserInterface|CreateWidget "/Game/StealthGame/Blueprints/Doors/W_OpenDoor.W_OpenDoor_C"))
    (UserInterface|Viewport|AddtoViewport _returnvalue 0)
    (else
      (bind _returnvalue_2 (UserInterface|CreateWidget "/Game/StealthGame/Blueprints/Doors/W_NeedKey.W_NeedKey_C"))
      (UserInterface|Viewport|AddtoViewport _returnvalue_2 0))))

(event OnComponentEndOverlap(Box)
  (params (OverlappedComponent :type Primitive%20Component%20Object%20Reference) (OtherActor :type Actor%20Object%20Reference) (OtherComp :type Primitive%20Component%20Object%20Reference) (OtherBodyIndex :type Integer))
  (Utilities|Casting|CastToBP_ThirdPersonCharacterCustom OtherActor)
  (if (Variables|Default|GetbHasKey?)
    (Widget|RemovefromParent (stale OnComponentBeginOverlap(Box) _returnvalue))
    (else
      (Widget|RemovefromParent (stale OnComponentBeginOverlap(Box) _returnvalue_2)))))

(event EventInteract
  (if (Variables|Default|GetbHasKey?)
    (Utilities|FlowControl|FlipFlop
      (:A
        (bind _door_track (Timeline|Door%20Timeline Play)
          (:Update
            (Transformation|SetRelativeRotation (Variables|Default|GetDoor) (Math|Rotator|MakeRotator 0.0 0.0 (Math|Float|Lerp 0.0 1.1e+02 _door_track)) false false))))
      (:B
        (Timeline|Door%20Timeline Reverse)))))

(event EventPickUpKey
  (Variables|Default|SetbHasKey? true))

(fn ConstructionScript)