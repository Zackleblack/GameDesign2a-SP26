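; BP_LibraryKey is a pickup key for the library that spins on a timeline-driven roll.
; Its box overlap with the custom third-person character sets NearKey and shows a pickup prompt widget, which is removed when the overlap ends.
; Interact notifies the referenced Door, plays a pickup sound, destroys the key, then sets KeyWasGot and displays a configurable widget.
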(event OnComponentBeginOverlap(Box)
  (params (OverlappedComponent :type Primitive%20Component%20Object%20Reference) (OtherActor :type Actor%20Object%20Reference) (OtherComp :type Primitive%20Component%20Object%20Reference) (OtherBodyIndex :type Integer) (bFromSweep :type Boolean) (SweepResult :type Hit%20Result%20Structure%20%28by%20ref%29))
  (Utilities|Casting|CastToBP_ThirdPersonCharacterCustom OtherActor)
  (Variables|Default|SetbNearKey? true)
  (bind _returnvalue (UserInterface|CreateWidget "/Game/StealthGame/Blueprints/Doors/W_Pickup.W_Pickup_C"))
  (UserInterface|Viewport|AddtoViewport _returnvalue 0))

(event OnComponentEndOverlap(Box)
  (params (OverlappedComponent :type Primitive%20Component%20Object%20Reference) (OtherActor :type Actor%20Object%20Reference) (OtherComp :type Primitive%20Component%20Object%20Reference) (OtherBodyIndex :type Integer))
  (Utilities|Casting|CastToBP_ThirdPersonCharacterCustom OtherActor)
  (Widget|RemovefromParent (stale OnComponentBeginOverlap(Box) _returnvalue)))

(event EventBeginPlay
  (bind _roation_time (Timeline|Rotation Play)
    (:Update
      (Transformation|SetRelativeRotation (Variables|Default|GetLibrary_Key_6BCE0292) (Math|Rotator|MakeRotator (Math|Float|Lerp 0.0 (Variables|Default|GetHow%20long%20spin?%20%28Y%29) _roation_time) -9e+01 0.0) false false))))

(event EventInteract
  ;[0.15 0.15 0.15 0.5] Interact Event - E
  (Class|BPIDoor|PickUpKey(Message) (Variables|Default|GetDoor))
  (Audio|PlaySound2D "/Game/StealthGame/Blueprints/Doors/KeyPickup_Cue.KeyPickup_Cue" 1.0 1.0 0.0 0 0)
  (Actor|DestroyActor)
  (Variables|Default|SetbKeyWasGot true)
  (bind _returnvalue (UserInterface|CreateWidget (Variables|Default|GetWidget%20Used)))
  (UserInterface|Viewport|AddtoViewport _returnvalue 0))

(fn ConstructionScript)