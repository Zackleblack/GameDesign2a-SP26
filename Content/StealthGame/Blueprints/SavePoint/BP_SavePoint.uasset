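; Save point actor for the stealth game that saves the game through the custom third-person character on overlap.
; A DoOnce-gated save plays a shutter sound, shows a temporary saved widget and spawns a Niagara effect.
; Timelines spin the point down, while a dynamic material turns the torus grey and the light hides.
; Leaving or re-entering after a save starts a retriggerable cooldown that restores spin, color and light and resets the gate.
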(event OnComponentBeginOverlap(Collision)
  (params (OverlappedComponent :type Primitive%20Component%20Object%20Reference) (OtherActor :type Actor%20Object%20Reference) (OtherComp :type Primitive%20Component%20Object%20Reference) (OtherBodyIndex :type Integer) (bFromSweep :type Boolean) (SweepResult :type Hit%20Result%20Structure%20%28by%20ref%29))
  ;[0.15 0.15 0.15 0.5] Comment
  (Development|PrintString "You hit Savepoint")
  (if (Variables|Default|GetbDidPlayerSave?)
    (CallFunction|SaveCooldown)
    (else
      (Utilities|FlowControl|DoOnce false
        (:Completed
          (Utilities|FlowControl|Sequence
            (:then_0
              (Audio|PlaySound2D "/Engine/VREditor/Sounds/UI/Camera_Shutter.Camera_Shutter" 1.0 1.0 0.0 0 0)
              (bind _returnvalue (UserInterface|CreateWidget "/Game/StealthGame/Core/W_GameSaved.W_GameSaved_C"))
              (UserInterface|Viewport|AddtoViewport _returnvalue 0)
              (Utilities|FlowControl|Delay 4.0)
              (Widget|RemovefromParent _returnvalue)
              (Variables|Default|SetbDidPlayerSave? true))
            (:then_1
              (bind _asbp_third_person_character_custom (Utilities|Casting|CastToBP_ThirdPersonCharacterCustom OtherActor))
              (Default|SaveGameState _asbp_third_person_character_custom)
              (CallFunction|SpeedUp/SlowDownSpin)
              (CallFunction|SavepointOffline))
            (:then_2
              (Niagara|SpawnSystematLocation "/Game/Developer/VFX/NS_Save.NS_Save" (Variables|/Script/Engine.SceneComponent|GetRelativeLocation (Variables|Default|GetDefaultSceneRoot)) "0, 0, 0" "1.000000,1.000000,1.000000" false))))))))

(event OnComponentEndOverlap(Collision)
  (params (OverlappedComponent :type Primitive%20Component%20Object%20Reference) (OtherActor :type Actor%20Object%20Reference) (OtherComp :type Primitive%20Component%20Object%20Reference) (OtherBodyIndex :type Integer))
  ;[0.15 0.15 0.15 0.5] Player has left Collision
  (Utilities|Casting|CastToBP_ThirdPersonCharacterCustom OtherActor)
  (Utilities|FlowControl|Delay 4.0)
  (Widget|RemovefromParent (stale OnComponentBeginOverlap(Collision) _returnvalue))
  (CallFunction|SaveCooldown))

(event Custom|Save%20Cooldown
  ;[0.15 0.15 0.15 0.5] Comment
  ;;[0.02278 0.04977 0.15 0.5] Saving Cooldown
  (Utilities|FlowControl|RetriggerableDelay 5.0)
  (Utilities|FlowControl|Sequence
    (:then_0
      (bind _time (Timeline|Timeline_0 Play)
        (:Update
          (Variables|/Script/Engine.RotatingMovementComponent|SetRotationRate (Variables|Default|GetRotatingMovement) (Math|Rotator|MakeRotator 0.0 0.0 (Math|Float|Lerp 0.0 1.8e+02 _time)))
          (CallFunction|ResetSound)
          (Variables|Default|SetbDidPlayerSave? false))))
    (:then_1
      (CallFunction|SavepointOnline))))

(event Custom|Reset%20Sound
  ;[0.15 0.15 0.15 0.5] Comment
  (Utilities|FlowControl|DoOnce false) ; enters at Reset
)

(event Custom|Speed%20Up%20/%20Slow%20Down%20Spin
  (bind _rotatingmovement (Variables|Default|GetRotatingMovement))
  ;[0.03855 0.03855 0.15 0.5] Speed Up / Slow Down Spin
  (Variables|/Script/Engine.RotatingMovementComponent|SetRotationRate _rotatingmovement "0.000000,360.000000,0.000000")
  (bind _time (Timeline|Timeline PlayFromStart)
    (:Update
      (Variables|/Script/Engine.RotatingMovementComponent|SetRotationRate _rotatingmovement (Math|Rotator|MakeRotator 0.0 0.0 (Math|Float|Lerp 3.6e+02 0.0 _time))))))

(event Custom|Savepoint%20Offline
  ;[0.15 0.15 0.15 0.5] Savepoint Offline
  (bind _returnvalue (Rendering|Material|CreateDynamicMaterialInstance (Variables|Default|GetTorus%20Point) 0 0 "None" :!class /Script/Engine.PrimitiveComponent))
  (bind _blue_to_grey (Timeline|Color%20Timeline PlayFromStart)
    (:Update
      (Rendering|Material|SetVectorParameterValue _returnvalue "Material Color" _blue_to_grey :!class /Script/Engine.MaterialInstanceDynamic)
      (Development|SetHiddeninGame (Variables|Default|GetLight) true false))))

(event Custom|Savepoint%20Online
  ;[0.15 0.15 0.15 0.5] Savepoint Online
  (bind _returnvalue (Rendering|Material|CreateDynamicMaterialInstance (Variables|Default|GetTorus%20Point) 0 0 "None" :!class /Script/Engine.PrimitiveComponent))
  (bind _grey_to_blue (Timeline|Timeline_1 PlayFromStart)
    (:Update
      (Rendering|Material|SetVectorParameterValue _returnvalue "Material Color" _grey_to_blue :!class /Script/Engine.MaterialInstanceDynamic)
      (Development|SetHiddeninGame (Variables|Default|GetLight) false false))))

(fn ConstructionScript)