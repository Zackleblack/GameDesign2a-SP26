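; Bookshelf puzzle actor that the player completes by placing a collected book, which removes a glass component.
; A trigger box shows a press-E or missing-book prompt to the custom third-person character, depending on whether the book is held.
; PickUpBook sets the held flag, which lets Interact reveal the hidden mesh, mark the shelf complete, destroy the glass, play a confirm sound and clear the prompt.
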(event OnComponentBeginOverlap(BoxCollision)
  (params (OverlappedComponent :type Primitive%20Component%20Object%20Reference) (OtherActor :type Actor%20Object%20Reference) (OtherComp :type Primitive%20Component%20Object%20Reference) (OtherBodyIndex :type Integer) (bFromSweep :type Boolean) (SweepResult :type Hit%20Result%20Structure%20%28by%20ref%29))
  (Utilities|Casting|CastToBP_ThirdPersonCharacterCustom OtherActor)
  (if (not (Variables|Default|GetbShelfIsComplete))
    (if (Variables|Default|GetbHasBook?)
      (bind _returnvalue (UserInterface|CreateWidget "/Game/StealthGame/Core/Characters/PlayerCharacter/W_PressE.W_PressE_C"))
      (UserInterface|Viewport|AddtoViewport _returnvalue 0)
      (else
        (bind _returnvalue_2 (UserInterface|CreateWidget "/Game/StealthGame/Blueprints/BookPuzzle/Widgets/W_MissingBook.W_MissingBook_C"))
        (UserInterface|Viewport|AddtoViewport _returnvalue_2 0)))))

(event OnComponentEndOverlap(BoxCollision)
  (params (OverlappedComponent :type Primitive%20Component%20Object%20Reference) (OtherActor :type Actor%20Object%20Reference) (OtherComp :type Primitive%20Component%20Object%20Reference) (OtherBodyIndex :type Integer))
  (Utilities|Casting|CastToBP_ThirdPersonCharacterCustom OtherActor)
  (if (Variables|Default|GetbHasBook?)
    (Widget|RemovefromParent (stale OnComponentBeginOverlap(BoxCollision) _returnvalue))
    (else
      (Widget|RemovefromParent (stale OnComponentBeginOverlap(BoxCollision) _returnvalue_2)))))

(event Custom|Destroy%20Glass
  (if (Variables|Default|GetbShelfIsComplete)
    (Components|DestroyComponent (Variables|Default|GetGlass))))

(event EventInteract
  (if (not (Variables|Default|GetbShelfIsComplete))
    (if (Variables|Default|GetbHasBook?)
      (Utilities|FlowControl|Sequence
        (:then_0
          (Development|SetHiddeninGame (Variables|Default|GetStaticMesh) false false)
          (Variables|Default|SetbShelfIsComplete true)
          (CallFunction|DestroyGlass)
          (Audio|PlaySound2D "/Engine/VREditor/Sounds/VR_confirm_Cue.VR_confirm_Cue" 1.0 1.0 0.0 0 0))
        (:then_1
          (Widget|RemovefromParent (stale OnComponentBeginOverlap(BoxCollision) _returnvalue)))))))

(event EventPickUpBook
  (Variables|Default|SetbHasBook? true))

(fn ConstructionScript)