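; BP_BookPuzzle is a collectible book pickup for a bookshelf puzzle.
; A Timeline started on BeginPlay spins the book in yaw, and box overlap with the player character adds or removes a press-E prompt widget.
; Interact notifies the referenced bookshelf through PickUpBookMessage, plays a pickup sound, destroys the actor and adds a placement widget to the viewport.
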(event OnComponentBeginOverlap(Box)
  (params (OverlappedComponent :type Primitive%20Component%20Object%20Reference) (OtherActor :type Actor%20Object%20Reference) (OtherComp :type Primitive%20Component%20Object%20Reference) (OtherBodyIndex :type Integer) (bFromSweep :type Boolean) (SweepResult :type Hit%20Result%20Structure%20%28by%20ref%29))
  (Utilities|Casting|CastToBP_ThirdPersonCharacterCustom OtherActor)
  (bind _returnvalue (UserInterface|CreateWidget "/Game/StealthGame/Core/Characters/PlayerCharacter/W_PressE.W_PressE_C"))
  (UserInterface|Viewport|AddtoViewport _returnvalue 0))

(event OnComponentEndOverlap(Box)
  (params (OverlappedComponent :type Primitive%20Component%20Object%20Reference) (OtherActor :type Actor%20Object%20Reference) (OtherComp :type Primitive%20Component%20Object%20Reference) (OtherBodyIndex :type Integer))
  (Utilities|Casting|CastToBP_ThirdPersonCharacterCustom OtherActor)
  (Widget|RemovefromParent (stale OnComponentBeginOverlap(Box) _returnvalue)))

(event EventBeginPlay
  (bind _rotation (Timeline|Timeline Play)
    (:Update
      (Transformation|SetRelativeRotation (Variables|Default|GetBook) (Math|Rotator|MakeRotator 0.0 0.0 (Math|Float|Lerp 0.0 3.6e+02 _rotation)) false false))))

(event EventInteract
  (Class|BPIPuzzleSlot|PickUpBook(Message) (Variables|Default|GetBookshelf%20Reference))
  (Audio|PlaySound2D "/Engine/VREditor/Sounds/UI/Object_PickUp.Object_PickUp" 1.0 1.0 0.0 0 0)
  (Actor|DestroyActor)
  (bind _returnvalue (UserInterface|CreateWidget (Variables|Default|GetWidget%20Placement) (Game|GetPlayerController 0)))
  (UserInterface|Viewport|AddtoViewport _returnvalue 0))

(fn ConstructionScript)