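; Blockout doorway actor for level prototyping, built procedurally from a configurable size and top and side thicknesses.
; The construction script calls rounding helpers on those dimensions using RoundSize, builds the doorway, then calls BlockoutSetMaterial.
; AddBlockoutDoorway adds left, top and right casings as copies of one mesh, scaled and offset to frame the opening, with sizes divided by 100 for scale.
; The event graph holds no active logic.
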(event EventBeginPlay)

(event Collision|EventActorBeginOverlap
  (params (OtherActor :type Actor%20Object%20Reference)))

(event EventTick
  (params (DeltaSeconds :type Float%20%28single-precision%29)))

(fn ConstructionScript
  (CallFunction|BlockoutRoundVector (Variables|BlockoutTools|BlockoutDoorway|GetbRoundSize) (Variables|BlockoutTools|BlockoutDoorway|GetDoorwaySize))
  (CallFunction|BlockoutRoundFloat (Variables|BlockoutTools|BlockoutDoorway|GetbRoundSize) (Variables|BlockoutTools|BlockoutDoorway|GetTopThickness))
  (CallFunction|BlockoutRoundFloat (Variables|BlockoutTools|BlockoutDoorway|GetbRoundSize) (Variables|BlockoutTools|BlockoutDoorway|GetSideThickness))
  (CallFunction|AddBlockoutDoorway)
  (Class|BlockoutToolsParent|BlockoutSetMaterial))

(fn AddBlockoutDoorway
  (bind _doorwaysize (Variables|BlockoutTools|BlockoutDoorway|GetDoorwaySize))
  (bind _doorwaysize_2 (Variables|BlockoutTools|BlockoutDoorway|GetDoorwaySize))
  (bind _doorwaysize_3 (Variables|BlockoutTools|BlockoutDoorway|GetDoorwaySize))
  (bind (_x _y _z) (Math|Vector|BreakVector _doorwaysize_3))
  (bind (_x_2 _y_2 _z_2) (Math|Vector|BreakVector _doorwaysize))
  (bind (_x_3 _y_3) (Math|Vector|BreakVector _doorwaysize_2))
  (bind _returnvalue (AddComponent|AddStaticMeshComponent false (Math|Transform|MakeTransform "0, 0, 0" "0, 0, 0" (* (Math|Vector|MakeVector _x (Variables|BlockoutTools|BlockoutDoorway|GetSideThickness) _z) (/ 1.0 1e+02))))) ; Casing Left
  (Components|StaticMesh|SetStaticMesh _returnvalue (Variables|BlockoutTools|BlockoutDoorway|GetBlockoutDoorwayMesh))
  (bind _returnvalue_2 (AddComponent|AddStaticMeshComponent false (Math|Transform|MakeTransform (Math|Vector|MakeVector 0.0 (Variables|BlockoutTools|BlockoutDoorway|GetSideThickness) (- (.Z (Math|Vector|BreakVector (Variables|BlockoutTools|BlockoutDoorway|GetDoorwaySize))) (Variables|BlockoutTools|BlockoutDoorway|GetTopThickness))) "0, 0, 0" (* (Math|Vector|MakeVector _x_3 (- _y_3 (* (Variables|BlockoutTools|BlockoutDoorway|GetSideThickness) 2.0)) (Variables|BlockoutTools|BlockoutDoorway|GetTopThickness)) (/ 1.0 1e+02))))) ; Casing Top
  (Components|StaticMesh|SetStaticMesh _returnvalue_2 (Variables|BlockoutTools|BlockoutDoorway|GetBlockoutDoorwayMesh))
  (bind _returnvalue_3 (AddComponent|AddStaticMeshComponent false (Math|Transform|MakeTransform (Math|Vector|MakeVector 0.0 (- (.Y (Math|Vector|BreakVector (Variables|BlockoutTools|BlockoutDoorway|GetDoorwaySize))) (Variables|BlockoutTools|BlockoutDoorway|GetSideThickness)) 0.0) "0, 0, 0" (* (Math|Vector|MakeVector _x_2 (Variables|BlockoutTools|BlockoutDoorway|GetSideThickness) _z_2) (/ 1.0 1e+02))))) ; Casing Right
  (Components|StaticMesh|SetStaticMesh _returnvalue_3 (Variables|BlockoutTools|BlockoutDoorway|GetBlockoutDoorwayMesh)))