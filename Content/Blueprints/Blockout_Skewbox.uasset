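; Blockout level-design actor that builds a skewed, tapered box shape.
; The construction script rounds the end offset and the start and end cross-section sizes by RoundSize, creates the mesh, then applies the blockout material.
; It deforms a box static mesh, picked by Alignment, with a spline mesh component, using the offset as end position and the sizes as start and end scales.
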(event EventBeginPlay)

(event Collision|EventActorBeginOverlap
  (params (OtherActor :type Actor%20Object%20Reference)))

(event EventTick
  (params (DeltaSeconds :type Float%20%28single-precision%29)))

(fn ConstructionScript
  (CallFunction|BlockoutRoundVector (Variables|BlockoutTools|BlockoutSkewbox|GetbRoundSize) (Variables|BlockoutTools|BlockoutSkewbox|GetSkewboxLenght))
  (CallFunction|BlockoutRoundVector2D (Variables|BlockoutTools|BlockoutSkewbox|GetbRoundSize) (Variables|BlockoutTools|BlockoutSkewbox|GetStartSize))
  (CallFunction|BlockoutRoundVector2D (Variables|BlockoutTools|BlockoutSkewbox|GetbRoundSize) (Variables|BlockoutTools|BlockoutSkewbox|GetEndSize))
  (CallFunction|AddBlockoutSkewbox)
  (Class|BlockoutToolsParent|BlockoutSetMaterial))

(fn AddBlockoutSkewbox
  (bind _returnvalue (AddComponent|AddSplineMeshComponent false))
  (Components|StaticMesh|SetStaticMesh _returnvalue (Utilities|Select :Index (Variables|BlockoutTools|BlockoutSkewbox|GetAlignment) :Option%200 "/Game/Meshes/SM_Blockout_Box.SM_Blockout_Box" :Option%201 "/Game/Meshes/SM_Blockout_Box_Centered.SM_Blockout_Box_Centered" :Option%202 "/Game/Meshes/SM_Blockout_Box_Right.SM_Blockout_Box_Right"))
  (SplineMesh|SetStartandEnd _returnvalue "0, 0, 0" "100.000000, 0, 0" (Variables|BlockoutTools|BlockoutSkewbox|GetSkewboxLenght) "100.000000, 0, 0" true :!class /Script/Engine.SplineMeshComponent)
  (SplineMesh|SetStartScale _returnvalue (/ (Variables|BlockoutTools|BlockoutSkewbox|GetStartSize) 1e+02) true :!class /Script/Engine.SplineMeshComponent)
  (SplineMesh|SetEndScale _returnvalue (/ (Variables|BlockoutTools|BlockoutSkewbox|GetEndSize) 1e+02) true :!class /Script/Engine.SplineMeshComponent))