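; Blockout cylinder actor for level prototyping, sized by radius and height and built entirely in the construction script.
; It rounds both dimensions by RoundSize, then adds a static mesh component scaled from centimeters, with the mesh picked from an array by CylinderQuality.
; Material setup is delegated to BlockoutSetMaterial, and the event graph has no active logic.
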(event EventBeginPlay)

(event Collision|EventActorBeginOverlap
  (params (OtherActor :type Actor%20Object%20Reference)))

(event EventTick
  (params (DeltaSeconds :type Float%20%28single-precision%29)))

(fn ConstructionScript
  (CallFunction|BlockoutRoundFloat (Variables|BlockoutTools|BlockoutCylinder|GetbRoundSize) (Variables|BlockoutTools|BlockoutCylinder|GetCylinderRadius))
  (CallFunction|BlockoutRoundFloat (Variables|BlockoutTools|BlockoutCylinder|GetbRoundSize) (Variables|BlockoutTools|BlockoutCylinder|GetCylinderHeight))
  (CallFunction|AddBlockoutCylinder)
  (Class|BlockoutToolsParent|BlockoutSetMaterial))

(fn AddBlockoutCylinder
  (bind _returnvalue (/ 1.0 1e+02))
  (bind _cylinderradius (Variables|BlockoutTools|BlockoutCylinder|GetCylinderRadius))
  (bind _returnvalue_2 (* _cylinderradius 2.0))
  (bind _returnvalue_3 (* _returnvalue_2 _returnvalue))
  (bind _returnvalue_4 (AddComponent|AddStaticMeshComponent false (Math|Transform|MakeTransform "0, 0, 0" "0, 0, 0" (Math|Vector|MakeVector _returnvalue_3 _returnvalue_3 (* (Variables|BlockoutTools|BlockoutCylinder|GetCylinderHeight) (/ 1.0 1e+02))))))
  (Components|StaticMesh|SetStaticMesh _returnvalue_4 (Utilities|Array|Get(acopy) (Variables|BlockoutTools|BlockoutCylinder|GetBlockoutCylinderMeshes) (Variables|BlockoutTools|BlockoutCylinder|GetCylinderQuality))))