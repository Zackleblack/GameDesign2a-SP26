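; Blockout sphere actor for level greyboxing, built entirely in the construction script with no runtime logic.
; It rounds the radius to a grid size, then adds a static mesh component scaled from that radius, converting centimetres to a 100-unit base mesh.
; The mesh is a sphere or hemisphere picked from arrays by a quality index, after which a shared blockout material is applied.
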(event EventBeginPlay)

(event Collision|EventActorBeginOverlap
  (params (OtherActor :type Actor%20Object%20Reference)))

(event EventTick
  (params (DeltaSeconds :type Float%20%28single-precision%29)))

(fn ConstructionScript
  (CallFunction|BlockoutRoundFloat (Variables|BlockoutTools|BlockoutSphere|GetbRoundSize) (Variables|BlockoutTools|BlockoutSphere|GetSphereRadius))
  (CallFunction|AddBlockoutSphere)
  (Class|BlockoutToolsParent|BlockoutSetMaterial))

(fn AddBlockoutSphere
  (bind _returnvalue (AddComponent|AddStaticMeshComponent false (Math|Transform|MakeTransform "0, 0, 0" "0, 0, 0" (Math|Conversions|ToVector(Float) (* (* (Variables|BlockoutTools|BlockoutSphere|GetSphereRadius) 2.0) (/ 1.0 1e+02))))))
  (Components|StaticMesh|SetStaticMesh _returnvalue (select (Variables|BlockoutTools|BlockoutSphere|GetbIsHemisphere) (Utilities|Array|Get(acopy) (Variables|BlockoutTools|BlockoutSphere|GetBlockoutHemisphereMeshes) (Variables|BlockoutTools|BlockoutSphere|GetSphereQuality)) (Utilities|Array|Get(acopy) (Variables|BlockoutTools|BlockoutSphere|GetBlockoutSphereMeshes) (Variables|BlockoutTools|BlockoutSphere|GetSphereQuality)))))