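; Blockout Box is a construction-time level blockout actor that builds a resizable box for greyboxing.
; Its construction script rounds BoxSize by RoundSize, then adds a static mesh component using BlockoutBoxMesh, scaled to one hundredth of BoxSize.
; A final blockout helper call sets the material.
; The event graph holds only disabled default events, so it has no runtime logic.
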(event EventBeginPlay)

(event Collision|EventActorBeginOverlap
  (params (OtherActor :type Actor%20Object%20Reference)))

(event EventTick
  (params (DeltaSeconds :type Float%20%28single-precision%29)))

(fn ConstructionScript
  (CallFunction|BlockoutRoundVector (Variables|BlockoutTools|BlockoutBox|GetbRoundSize) (Variables|BlockoutTools|BlockoutBox|GetBoxSize))
  (CallFunction|AddBlockoutBox)
  (Class|BlockoutToolsParent|BlockoutSetMaterial))

(fn AddBlockoutBox
  (bind _returnvalue (AddComponent|AddStaticMeshComponent false (Math|Transform|MakeTransform "0, 0, 0" "0, 0, 0" (* (Variables|BlockoutTools|BlockoutBox|GetBoxSize) (/ 1.0 1e+02)))))
  (Components|StaticMesh|SetStaticMesh _returnvalue (Variables|BlockoutTools|BlockoutBox|GetBlockoutBoxMesh)))