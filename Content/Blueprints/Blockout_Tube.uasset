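; Blockout actor that builds a tube or arc wall for level prototyping, entirely in its construction script.
; It rounds the dimensions, then lays clamped spline points along a circle by radius, angle and section count, closing the loop at 360 degrees.
; Each segment gets a spline mesh box, chosen by alignment and scaled to thickness and height, before the blockout material is applied.
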(event EventBeginPlay)

(event Collision|EventActorBeginOverlap
  (params (OtherActor :type Actor%20Object%20Reference)))

(event EventTick
  (params (DeltaSeconds :type Float%20%28single-precision%29)))

(fn ConstructionScript
  (CallFunction|BlockoutRoundFloat (Variables|BlockoutTools|BlockoutTube|GetbRoundSize) (Variables|BlockoutTools|BlockoutTube|GetAngle))
  (CallFunction|BlockoutRoundFloat (Variables|BlockoutTools|BlockoutTube|GetbRoundSize) (Variables|BlockoutTools|BlockoutTube|GetRadius))
  (CallFunction|BlockoutRoundFloat (Variables|BlockoutTools|BlockoutTube|GetbRoundSize) (Variables|BlockoutTools|BlockoutTube|GetHeight))
  (CallFunction|BlockoutRoundFloat (Variables|BlockoutTools|BlockoutTube|GetbRoundSize) (Variables|BlockoutTools|BlockoutTube|GetThickness))
  (CallFunction|SetupSplineCircle)
  (CallFunction|AddBlockoutTube)
  (Class|BlockoutToolsParent|BlockoutSetMaterial))

(fn AddBlockoutTube
  (for _index (range 0 (- (Spline|GetNumberOfSplinePoints (Variables|Default|GetSpline)) 3))
    (bind _returnvalue (AddComponent|AddSplineMeshComponent false))
    (Components|StaticMesh|SetStaticMesh _returnvalue (Utilities|Select :Index (Variables|BlockoutTools|BlockoutTube|GetAlignment) :Option%200 "/Game/Meshes/SM_Blockout_Box.SM_Blockout_Box" :Option%201 "/Game/Meshes/SM_Blockout_Box_Centered.SM_Blockout_Box_Centered" :Option%202 "/Game/Meshes/SM_Blockout_Box_Right.SM_Blockout_Box_Right"))
    (SplineMesh|SetStartandEnd _returnvalue (.Location (Spline|GetLocationandTangentatSplinePoint (Variables|Default|GetSpline) _index "Local")) (select (== _index 0) "100.000000, 0, 0" (.Tangent (Spline|GetLocationandTangentatSplinePoint (Variables|Default|GetSpline) _index "Local"))) (.Location (Spline|GetLocationandTangentatSplinePoint (Variables|Default|GetSpline) (+ _index 1) "Local")) (.Tangent (Spline|GetLocationandTangentatSplinePoint (Variables|Default|GetSpline) (+ _index 1) "Local")) true :!class /Script/Engine.SplineMeshComponent)
    (SplineMesh|SetStartScale _returnvalue (/ (Math|Vector2D|MakeVector2D (Variables|BlockoutTools|BlockoutTube|GetThickness) (Variables|BlockoutTools|BlockoutTube|GetHeight)) 1e+02) true :!class /Script/Engine.SplineMeshComponent)
    (SplineMesh|SetEndScale _returnvalue (/ (Math|Vector2D|MakeVector2D (Variables|BlockoutTools|BlockoutTube|GetThickness) (Variables|BlockoutTools|BlockoutTube|GetHeight)) 1e+02) true :!class /Script/Engine.SplineMeshComponent)))

(fn SetupSplineCircle
  (Variables|BlockoutTools|BlockoutTube|SetSplinePoints (+ (Variables|BlockoutTools|BlockoutTube|GetSections) 1))
  (Spline|ClearSplinePoints (Variables|Default|GetSpline) true)
  (for _index (range 0 (Variables|BlockoutTools|BlockoutTube|GetSplinePoints))
    (Spline|SetSplinePointType (Variables|Default|GetSpline) _index "CurveClamped" true)
    (Spline|AddSplinePoint (Variables|Default|GetSpline) (* (Math|Vector|MakeVector (Math|Trig|Sin(Degrees) (* _index (/ (Variables|BlockoutTools|BlockoutTube|GetAngle) (Math|Conversions|ToFloat(Integer) (- (Variables|BlockoutTools|BlockoutTube|GetSplinePoints) 1))))) (Math|Trig|Cos(Degrees) (* _index (/ (Variables|BlockoutTools|BlockoutTube|GetAngle) (Math|Conversions|ToFloat(Integer) (- (Variables|BlockoutTools|BlockoutTube|GetSplinePoints) 1))))) 0.0) (Variables|BlockoutTools|BlockoutTube|GetRadius)) "Local" true))
  (if (== (Variables|BlockoutTools|BlockoutTube|GetAngle) 3.6e+02)
    (Spline|SetClosedLoop (Variables|Default|GetSpline) true true)
    (else
      (Spline|SetClosedLoop (Variables|Default|GetSpline) false true))))