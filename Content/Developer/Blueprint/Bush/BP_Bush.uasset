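; BP_Bush is a bush actor that crouches the custom third-person character and flags it as inside while it overlaps the InBushBox volume.
; Entering plays a shaking sound and Niagara effect at the character's mesh, then calls Crouch and EnteredBush.
; Exiting replays both effects and calls UnCrouch and ExitBush.
; A second exit cast to BP_ThirdPersonCharacter re-enters that branch, still targeting the custom-character cast result.
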(event OnComponentBeginOverlap(InBushBox)
  (params (OverlappedComponent :type Primitive%20Component%20Object%20Reference) (OtherActor :type Actor%20Object%20Reference) (OtherComp :type Primitive%20Component%20Object%20Reference) (OtherBodyIndex :type Integer) (bFromSweep :type Boolean) (SweepResult :type Hit%20Result%20Structure%20%28by%20ref%29))
  (Utilities|FlowControl|Sequence
    (:then_0
      (bind _asbp_third_person_character_custom (Utilities|Casting|CastToBP_ThirdPersonCharacterCustom OtherActor))
      (Audio|PlaySoundatLocation "/Game/Developer/Blueprint/Bush/Bush_Shaking.Bush_Shaking" (Transformation|GetWorldLocation (Variables|/Script/Engine.Character|GetMesh _asbp_third_person_character_custom)) "0, 0, 0" 1.0 1.0 0.0 0 0 0 0)
      (Niagara|SpawnSystematLocation "/Game/Developer/VFX/Footsteps/NS_Bush.NS_Bush" (Transformation|GetWorldLocation (Variables|/Script/Engine.Character|GetMesh _asbp_third_person_character_custom)))
      (Character|Crouch _asbp_third_person_character_custom))
    (:then_1
      (bind _asbp_third_person_character_custom_2 (Utilities|Casting|CastToBP_ThirdPersonCharacterCustom OtherActor))
      (Default|EnteredBush _asbp_third_person_character_custom_2))))

(event OnComponentEndOverlap(InBushBox)
  (params (OverlappedComponent :type Primitive%20Component%20Object%20Reference) (OtherActor :type Actor%20Object%20Reference) (OtherComp :type Primitive%20Component%20Object%20Reference) (OtherBodyIndex :type Integer))
  (Utilities|FlowControl|Sequence
    (:then_0
      (bind _asbp_third_person_character_custom (Utilities|Casting|CastToBP_ThirdPersonCharacterCustom OtherActor)))
    (:then_1
      (Utilities|Casting|CastToBP_ThirdPersonCharacter OtherActor)))
  (Utilities|FlowControl|Sequence
    (:then_0
      (Audio|PlaySoundatLocation "/Game/Developer/Blueprint/Bush/Bush_Shaking.Bush_Shaking" (Transformation|GetWorldLocation (Variables|/Script/Engine.Character|GetMesh _asbp_third_person_character_custom)) "0, 0, 0" 1.0 1.0 0.0 0 0 0 0)
      (Niagara|SpawnSystematLocation "/Game/Developer/VFX/Footsteps/NS_Bush.NS_Bush" (Transformation|GetWorldLocation (Variables|/Script/Engine.Character|GetMesh _asbp_third_person_character_custom)))
      (Character|UnCrouch _asbp_third_person_character_custom)
      (Default|ExitBush _asbp_third_person_character_custom))))

(fn ConstructionScript)