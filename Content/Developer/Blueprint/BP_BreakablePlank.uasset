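; BP_BreakablePlank is a plank that breaks when a BP_DistractionItemPawn overlaps its BreakHitbox.
; The first such overlap spawns the NS_Landing Niagara effect and plays a wood crate sound at the plank's location, then destroys the Plank component.
; DoOnce gates keep both steps from repeating.
; The actor itself is not destroyed, and the Delay after the break leads to nothing.
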(event OnComponentBeginOverlap(BreakHitbox)
  (params (OverlappedComponent :type Primitive%20Component%20Object%20Reference) (OtherActor :type Actor%20Object%20Reference) (OtherComp :type Primitive%20Component%20Object%20Reference) (OtherBodyIndex :type Integer) (bFromSweep :type Boolean) (SweepResult :type Hit%20Result%20Structure%20%28by%20ref%29))
  (bind _plank (Variables|Default|GetPlank))
  (bind _returnvalue (Transformation|GetWorldLocation _plank))
  (Utilities|Casting|CastToBP_DistractionItemPawn OtherActor)
  (Utilities|FlowControl|Sequence
    (:then_0
      (Utilities|FlowControl|DoOnce false
        (:Completed
          (Niagara|SpawnSystematLocation "/Game/Developer/VFX/Footsteps/NS_Landing.NS_Landing" _returnvalue)
          (Audio|PlaySoundatLocation "/Game/Developer/Blueprint/WoodCrate_Cue.WoodCrate_Cue" _returnvalue "0, 0, 0" 1.0 1.0 0.0 0 0 0 0))))
    (:then_1
      (Utilities|FlowControl|DoOnce false
        (:Completed
          (Components|DestroyComponent (Variables|Default|GetPlank))
          (Utilities|FlowControl|Delay 3.0))))))

(event EventBeginPlay)

(fn ConstructionScript)